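; ResistenceWall_BP is a wall actor that gives its cube mesh a random color when constructed.
; The construction script creates a dynamic instance of ResistenceWall_MT, calls CreateRandColor, and applies the result to the BaseColor parameter.
; CreateRandColor rolls each RGB channel in tenth steps from zero to one and stores it in ColorToPass.
; The event graph has no active gameplay logic.
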(event EventBeginPlay)

(event Collision|EventActorBeginOverlap
  (params (OtherActor :type Actor%20Object%20Reference)))

(event EventTick
  (params (DeltaSeconds :type Float%20%28single-precision%29)))

(fn ConstructionScript
  (bind _returnvalue (Rendering|Material|CreateDynamicMaterialInstance (Variables|Default|GetCube) 0 "/Game/Environment/Materials/ResistenceWall_MT.ResistenceWall_MT" :!class /Script/Engine.PrimitiveComponent))
  (CallFunction|CreateRandColor)
  (Rendering|Material|SetVectorParameterValue _returnvalue "BaseColor" (Variables|Default|GetColorToPass) :!class /Script/Engine.MaterialInstanceDynamic))

(fn CreateRandColor
  (Variables|Default|SetRed (/ (Math|Conversions|ToFloat(Integer) (Math|Random|RandomIntegerinRange 0 10)) 1e+01))
  (Variables|Default|SetGreen (/ (Math|Conversions|ToFloat(Integer) (Math|Random|RandomIntegerinRange 0 10)) 1e+01))
  (Variables|Default|SetBlue (/ (Math|Conversions|ToFloat(Integer) (Math|Random|RandomIntegerinRange 0 10)) 1e+01))
  (Variables|Default|SetColorToPass (Utilities|Struct|MakeLinearColor (Variables|Default|GetRed) (Variables|Default|GetGreen) (Variables|Default|GetBlue) 0.0)))