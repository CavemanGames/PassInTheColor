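; Player ship Blueprint for a colour-matching game where picked-up colours decide which resistance walls the ship can pass.
; Overlapping a colour pickup adds a step to its first bright RGB channel, or subtracts from all three for white, then clamps and destroys the pickup.
; The result drives BaseColor on the ship's dynamic material.
; A wall matching all three channels within a tolerance loses its collision; a mismatch pauses the game.
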(event OnComponentBeginOverlap(Ship)
  (params (OverlappedComponent :type Primitive%20Component%20Object%20Reference) (OtherActor :type Actor%20Object%20Reference) (OtherComp :type Primitive%20Component%20Object%20Reference) (OtherBodyIndex :type Integer) (bFromSweep :type Boolean) (SweepResult :type Hit%20Result%20Structure%20%28by%20ref%29))
  (bind _ascolor_to_spawn_bp (Utilities|Casting|CastToColorToSpawn_BP OtherActor)
    (:then
      (bind _colottoset (CallFunction|AddColoursPoint (Variables|/Game/Environment/Behaviour/ColorToSpawn_BP.ColorToSpawn_BP_C|GetColorToSet _ascolor_to_spawn_bp)))
      (Actor|DestroyActor _ascolor_to_spawn_bp)
      (Rendering|Material|SetVectorParameterValue (Variables|Default|GetPlayerColor) "BaseColor" _colottoset :!class /Script/Engine.MaterialInstanceDynamic))
    (:CastFailed
      (bind _asresistence_wall_bp (Utilities|Casting|CastToResistenceWall_BP OtherActor))
      (if (Math|Boolean|ANDBoolean (Math|Float|NearlyEqual(Float) (Variables|/Game/Environment/Behaviour/ResistenceWall_BP.ResistenceWall_BP_C|GetRed _asresistence_wall_bp) (Variables|Default|GetRedColor) 0.05) (Math|Float|NearlyEqual(Float) (Variables|/Game/Environment/Behaviour/ResistenceWall_BP.ResistenceWall_BP_C|GetGreen _asresistence_wall_bp) (Variables|Default|GetGreenColor) 0.05) (Math|Float|NearlyEqual(Float) (Variables|/Game/Environment/Behaviour/ResistenceWall_BP.ResistenceWall_BP_C|GetBlue _asresistence_wall_bp) (Variables|Default|GetBlueColor) 0.05))
        (Collision|SetActorEnableCollision _asresistence_wall_bp false)
        (else
          (Game|SetGamePaused true))))))

(event EventBeginPlay
  (bind _returnvalue (Rendering|Material|CreateDynamicMaterialInstance (Variables|Default|GetShip) 0 "/Game/Player/Material/PlayerMaterial.PlayerMaterial" :!class /Script/Engine.PrimitiveComponent))
  (Variables|Default|SetPlayerColor _returnvalue))

(event EventTick
  (params (DeltaSeconds :type Float%20%28single-precision%29)))

(fn ConstructionScript)

(fn AddColoursPoint
  (params (ObjectColor :type Linear%20Color%20Structure))
  (bind (_r _g _b) (Utilities|Struct|BreakLinearColor ObjectColor))
  (bind _returnvalue (> _b 0.5))
  (bind _returnvalue_2 (> _r 0.5))
  (bind _returnvalue_3 (> _g 0.5))
  (if (Math|Boolean|ANDBoolean _returnvalue_2 _returnvalue_3 _returnvalue)
    (Variables|Default|SetRedColor (- (Variables|Default|GetRedColor) (Variables|Default|GetColorValueToAdd)))
    (Variables|Default|SetGreenColor (- (Variables|Default|GetGreenColor) (Variables|Default|GetColorValueToAdd)))
    (Variables|Default|SetBlueColor (- (Variables|Default|GetBlueColor) (Variables|Default|GetColorValueToAdd)))
    (CallFunction|ClampAllColors :!label _label)
    (return (Utilities|Struct|MakeLinearColor (Variables|Default|GetRedColor) (Variables|Default|GetGreenColor) (Variables|Default|GetBlueColor) 0.0))
    (elif _returnvalue_2
      (Variables|Default|SetRedColor (+ (Variables|Default|GetRedColor) (Variables|Default|GetColorValueToAdd)))
      (goto _label)
      (elif _returnvalue_3
        (Variables|Default|SetGreenColor (+ (Variables|Default|GetGreenColor) (Variables|Default|GetColorValueToAdd)))
        (goto _label)
        (elif _returnvalue
          (Variables|Default|SetBlueColor (+ (Variables|Default|GetBlueColor) (Variables|Default|GetColorValueToAdd)))
          (goto _label))))))

(fn ClampAllColors
  (Variables|Default|SetRedColor (Math|Float|Clamp(Float) (Variables|Default|GetRedColor)))
  (Variables|Default|SetGreenColor (Math|Float|Clamp(Float) (Variables|Default|GetGreenColor)))
  (Variables|Default|SetBlueColor (Math|Float|Clamp(Float) (Variables|Default|GetBlueColor))))