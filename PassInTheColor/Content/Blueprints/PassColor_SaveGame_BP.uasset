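; SaveGame Blueprint for PassColor that holds a leaderboard of the five highest score entries.
; AddHighestScore appends a new entry to SaveStructure, calls SortSaveData, then trims the array to at most five.
; SortSaveData is a selection sort, repeatedly moving the DetermineHighestScoreValue result into a temporary array for descending order.
; DetermineLowestScoreValue returns the weakest entry and its index, but nothing in this Blueprint calls it.
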(fn DetermineLowestScoreValue
  (bind _savestructure (Variables|Default|GetSaveStructure))
  (if (> (Utilities|Array|Length _savestructure) 0)
    (for (_array_element _array_index) _savestructure
      (if (== _array_index 0)
        (LocalVariables|SetLowestScore (.score _array_element))
        (LocalVariables|SetLowestIndex _array_index)
        (elif (< (.score _array_element) (LocalVariables|GetLowestScore))
          (LocalVariables|SetLowestScore (.score _array_element))
          (LocalVariables|SetLowestIndex _array_index))))
    (return (Utilities|Array|Get(acopy) _savestructure (LocalVariables|GetLowestIndex)) (LocalVariables|GetLowestIndex))))

(fn DetermineHighestScoreValue
  (bind _savestructure (Variables|Default|GetSaveStructure))
  (for (_array_element _array_index) _savestructure
    (if (== _array_index 0)
      (LocalVariables|SetHighestScore (.score _array_element))
      (LocalVariables|SetHighestIndex _array_index)
      (elif (> (.score _array_element) (LocalVariables|GetHighestScore))
        (LocalVariables|SetHighestScore (.score _array_element))
        (LocalVariables|SetHighestIndex _array_index))))
  (return (Utilities|Array|Get(acopy) _savestructure (LocalVariables|GetHighestIndex)) (LocalVariables|GetHighestIndex)))

(fn SortSaveData
  (while (> (Utilities|Array|Length (Variables|Default|GetSaveStructure)) 0)
    (bind (_lowestscorestruct _lowestscoreindex) (CallFunction|DetermineHighestScoreValue))
    (Utilities|Array|Add (LocalVariables|GetTempStruct) _lowestscorestruct)
    (Utilities|Array|RemoveIndex (Variables|Default|GetSaveStructure) _lowestscoreindex))
  (Variables|Default|SetSaveStructure (LocalVariables|GetTempStruct)))

(fn AddHighestScore
  (params (NewScore :type Hight%20Score%20Structure%20Structure))
  (bind _savestructure (Variables|Default|GetSaveStructure))
  (Utilities|Array|Add (Variables|Default|GetSaveStructure) NewScore)
  (CallFunction|SortSaveData)
  (Utilities|Array|Resize _savestructure (Math|Integer|Min(Integer) (Utilities|Array|Length _savestructure) 5)))