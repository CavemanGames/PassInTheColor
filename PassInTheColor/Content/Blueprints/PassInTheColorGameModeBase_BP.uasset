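; Game mode for the Pass In The Color game that provides the high-score save game and the sound-enabled setting.
; CreateLoadGame loads and sorts the existing high-score slot, or creates a new save object in memory if none exists, then caches and returns it.
; SoundEnabled is read from the save's lowest-score struct rather than a separate setting.
; BeginPlay is empty, so CreateLoadGame is not called within this Blueprint.
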(event EventBeginPlay)

(fn ConstructionScript)

(fn CreateLoadGame
  (bind _returnvalue (SaveGame|DoesSaveGameExist (Variables|Default|GetHightScoreSaveGame)))
  (if _returnvalue
    (bind _returnvalue_2 (SaveGame|LoadGamefromSlot (Variables|Default|GetHightScoreSaveGame)))
    (bind _aspass_color_save_game_bp (Utilities|Casting|CastToPassColor_SaveGame_BP _returnvalue_2)
      (:then
        (Default|SortSaveData _aspass_color_save_game_bp)
        (bind _output_get (Variables|Default|SetCurrentSaveGame _aspass_color_save_game_bp))
        (bind _lowestscorestruct (Default|DetermineLowestScoreValue _output_get :!label _label))
        (Variables|Default|SetSoundEnabled (.soundenabled _lowestscorestruct))
        (return (Variables|Default|GetCurrentSaveGame)))
      (:CastFailed
        _))
    (else
      (bind _returnvalue_3 (SaveGame|CreateSaveGameObject "/Game/Blueprints/PassColor_SaveGame_BP.PassColor_SaveGame_BP_C"))
      (Utilities|IsValid _returnvalue_3
        (:Is%20Valid
          (Variables|Default|SetCurrentSaveGame _returnvalue_3)
          (goto _label))
        (:Is%20Not%20Valid
          _))))
  (return 0))

(fn NewFunction0)